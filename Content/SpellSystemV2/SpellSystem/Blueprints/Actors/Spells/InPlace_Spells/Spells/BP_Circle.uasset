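; BP_Circle is an in-place spell actor that releases a burst of mini energy balls above a fading circle decal.
; On BeginPlay the server snaps it to a downward trace from the instigator and calls StartTimer.
; StartTimer spawns randomly rotated balls above the pre-snap location, splitting the spell's Value among them.
; Timelines scale and fade in the decal, then after a delay deactivate Niagara, reverse the fade and destroy the actor.
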(event `self.ReceiveBeginPlay`
  (bind _instigator (`self.Instigator`))
  (bind _returnvalue (`self.K2_GetActorLocation` _instigator))
  ;[0 0 0] Begin Play
  (`parent.ReceiveBeginPlay`)
  (if (`KismetSystemLibrary.IsServer`)
    (`SceneComponent.K2_SetWorldRotation` :`self` (`self.Sphere`))
    (set `self.SpawnLocation` (`SceneComponent.K2_GetComponentLocation` (`self.Sphere`)))
    (`self.Start Timer`)
    (bind _outhit (`KismetSystemLibrary.LineTraceSingle` _returnvalue (+ _returnvalue (* (`self.GetActorUpVector` _instigator) -222.0)) "TraceTypeQuery1"))
    (`self.K2_SetActorLocation` (`.Location` (`GameplayStatics.BreakHitResult` _outhit)))))

(event `Spawn Projectile`
  (bind (_spawnlocation_x _spawnlocation_y _spawnlocation_z) (`KismetMathLibrary.BreakVector` (`self.SpawnLocation`)))
  ;[0 0 0] Spawn Projectiles
  (`|SpawnActorFromClass` "/Game/SpellSystemV2/SpellSystem/Blueprints/Actors/Spells/Damage_Spells/Spells/BP_MiniEnergyBall.BP_MiniEnergyBall_C" (`KismetMathLibrary.MakeTransform` (`KismetMathLibrary.MakeVector` _spawnlocation_x _spawnlocation_y (+ _spawnlocation_z 255.0)) (`self.Rotation`)) "Undefined" "OverrideRootScale" null (/ (`self.Value`) (`self.Number of Balls`)) false "Ball" (`self.Instigator`)))

(event `Start Timer`
  ;[0 0 0] Spawn Decal / Set Decal Opacity / Set Timer
  (bind _returnvalue (`DecalComponent.CreateDynamicMaterialInstance` (`self.Decal`)))
  (set `self.Forward` true)
  (`|ExecutionSequence`
    (:`then_0`
      (`|ExecutionSequence`
        (:`then_0`
          ;[0 0 0] Spawn Projectiles
          (if (`KismetSystemLibrary.IsServer`)
            (for _ (range (+ (`self.Number of Balls`) 1))
              (set `self.Rotation` (`KismetMathLibrary.MakeRotator` (`KismetMathLibrary.RandomFloatInRange` -60.0 60.0) (`KismetMathLibrary.RandomFloatInRange` -60.0 60.0) (`KismetMathLibrary.RandomFloatInRange` -360.0 360.0)))
              (`self.Spawn Projectile`))))
        (:`then_1`
          (bind (_direction _newtrack_1) (`Timeline|Timeline_0`)
            (:`Update`
              (`SceneComponent.SetRelativeScale3D` (`self.Decal`) (`KismetMathLibrary.MakeVector` 1.0 _newtrack_1 _newtrack_1)))))))
    (:`then_1`
      (bind (_direction_2 _opacity) (`Timeline|Timeline` :!label _label)
        (:`Update`
          (`MaterialInstanceDynamic.SetScalarParameterValue` _returnvalue "Opacity" _opacity))
        (:`Finished`
          (if (`self.Forward`)
            (`KismetSystemLibrary.K2_SetTimerDelegate` (delegate `CustomEvent`) 2.0)
            (else
              (`self.K2_DestroyActor`))))))))

(event `CustomEvent`
  ;[0 0 0] Spawn Decal / Set Decal Opacity / Set Timer
  (`ActorComponent.Deactivate` (`self.Niagara`))
  (set `self.Forward` false)
  (goto _label :!via `Reverse`))

(fn `UserConstructionScript`
  (`parent.UserConstructionScript`))