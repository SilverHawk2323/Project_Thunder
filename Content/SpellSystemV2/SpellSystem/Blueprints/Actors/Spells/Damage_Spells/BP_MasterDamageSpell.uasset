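; Base damage spell actor that plays a looping Niagara effect and damages what its sphere touches.
; Overlap and hit events share one path that ignores the owner and same-instigator actors, then stops the effect and disables collision.
; The server applies standard damage and sends a TakeDamage message with forced interrupt.
; Non-dedicated instances spawn the impact effect and destroy the actor when it finishes.
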(event `self.ReceiveBeginPlay`
  ;[0 0 0] Begin Play
  (`NiagaraComponent.SetAsset` (`self.Niagara`) (`self.System - Loop`) true))

(event `self.Sphere.OnComponentBeginOverlap`
  (params (OverlappedComponent :type "PrimitiveComponent Object Reference") (OtherActor :type "Actor Object Reference") (OtherComp :type "PrimitiveComponent Object Reference") (OtherBodyIndex :type Integer) (bFromSweep :type Boolean) (SweepResult :type "HitResult Structure (by ref)"))
  (bind _value (`self.Value`))
  ;[0 0 0] Hit
  (set `self.HitActor` OtherActor)
  (if (!= (`self.GetOwner`) (`self.HitActor`)) :!label _label
    (if (not (== (`self.GetInstigator` (`self.HitActor`)) (`self.GetInstigator`)))
      (`ActorComponent.Deactivate` (`self.Niagara`))
      (`PrimitiveComponent.SetCollisionEnabled` (`self.Sphere`) "NoCollision")
      (if (not (`KismetSystemLibrary.IsDedicatedServer`))
        (bind _returnvalue (`NiagaraFunctionLibrary.SpawnSystemAtLocation` (`self.System - Hit`) (`self.K2_GetActorLocation`)))
        (add `NiagaraComponent.OnSystemFinished` _returnvalue (delegate `CustomEvent`)))
      (if (or (`KismetSystemLibrary.IsServer`) (`KismetSystemLibrary.IsDedicatedServer`))
        (`GameplayStatics.ApplyDamage` (`self.HitActor`) _value null (`self.Instigator`))
        (bind _hitactor (`self.HitActor`)
          (:`then`
            (message `/Game/Blueprint/DamageSystem/BPI_Damageable.TakeDamage` _hitactor (make `/Game/Blueprint/DamageSystem/S_DamageInfo` _value "NewEnumerator2" "NewEnumerator1" false false false true) (`self.Instigator`)))
          (:`else`))))))

(event `self.Sphere.OnComponentHit`
  (params (HitComponent :type "PrimitiveComponent Object Reference") (OtherActor :type "Actor Object Reference") (OtherComp :type "PrimitiveComponent Object Reference") (NormalImpulse :type "Vector Structure") (Hit :type "HitResult Structure (by ref)"))
  ;[0 0 0] Hit
  (set `self.HitActor` OtherActor)
  (goto _label))

(event `CustomEvent`
  (params (PSystem :type "NiagaraComponent Object Reference"))
  ;[0 0 0] Hit
  (remove `NiagaraComponent.OnSystemFinished` (stale `self.Sphere.OnComponentBeginOverlap` _returnvalue) (delegate `CustomEvent`))
  (`self.K2_DestroyActor`))

(fn `UserConstructionScript`)