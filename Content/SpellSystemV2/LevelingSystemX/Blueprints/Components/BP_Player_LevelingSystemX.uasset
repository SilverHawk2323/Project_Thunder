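; Player character component that handles experience, levels, rank points and an overhead name, level and rank widget.
; Server events scale experience by reward versus character level, loop through level-ups, set SpellSystem_Component spell points and trigger multicast effects.
; OnRep functions refresh the screen-space widget, and rank point changes are batched through a retriggerable delay.
; A locally created overlap sphere fades nearby players' widgets; an example sphere-damage attack is included.
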(event `Leveling Up (Visual Effect) - Server`
  ;[0 0 0] Leveling Up - Spawn Effect
  (`self.Leveling Up (Visual Effect) - Multicast`))

(event `Leveling Up (Visual Effect) - Multicast`
  ;[0 0 0] Leveling Up - Spawn Effect
  (bind _returnvalue (`|SpawnActorFromClass` "/Game/SpellSystemV2/LevelingSystemX/Blueprints/Actors/BP_LevelUP.BP_LevelUP_C" (`KismetMathLibrary.MakeTransform` (`KismetMathLibrary.MakeVector` 0.0 0.0 (* (`CapsuleComponent.CapsuleHalfHeight` (`Character.CapsuleComponent` (`self.As Character`))) -1.0))) "Undefined" "OverrideRootScale" null null))
  (`Actor.K2_AttachToActor` _returnvalue (`self.As Character`) "root" "KeepRelative" "KeepRelative" "KeepRelative" true)
  (`SceneComponent.SetAbsolute` (`Actor.RootComponent` _returnvalue) false true false))

(event `Set Name - Server`
  ;[0 0 0] Set Player Name
  (bind _player_name (`/Game/SpellSystemV2/LevelingSystemX/Blueprints/BP_Components_MacroLib.Get Player Player Name` 15.0 (`self.As Character`))
    (:`Is Valid`
      (set `self.Player Name` (`KismetStringLibrary.Conv_StringToName` _player_name)))))

(event `Set Name`
  (params (`Player Name` :type Name))
  ;[0 0 0] Set Player Name
  (bind _level_and_rank___widget (`/Game/SpellSystemV2/LevelingSystemX/Blueprints/BP_Components_MacroLib.Get Level And Rank - Widget` 15.0 self)
    (:`Is Valid`
      (bind _aswb_player_level_attached (cast `/Game/SpellSystemV2/LevelingSystemX/Blueprints/Widgets/WB_PlayerLevel_Attached` (`WidgetComponent.GetUserWidgetObject` _level_and_rank___widget)))
      (`/Game/SpellSystemV2/LevelingSystemX/Blueprints/Widgets/WB_PlayerLevel_Attached.Set Player Name` _aswb_player_level_attached `Player Name`))))

(event `self.ReceiveBeginPlay`
  ;[0 0 0] Begin Play
  (bind _ascharacter (cast `Character` (`self.GetOwner`)))
  (set `self.As Character` _ascharacter)
  (if (not (`KismetSystemLibrary.IsDedicatedServer`))
    (`self.Set Level and Rank - Widget`)
    (`|ExecutionSequence`
      (:`then_0`
        ;[0 0 0] Disable Tick For Widget Component
        (`KismetSystemLibrary.Delay` 0.2)
        (`self.SetComponentTickEnabled` (`self.Level and Rank - Widget`) false))
      (:`then_1`
        (if (`Pawn.IsLocallyControlled` (`self.As Character`))
          (`self.Set Name - Server`)
          (`self.Set Collision`))))))

(event `Refreshing Rank Points`
  ;[0 0 0] Refreshing Rank Points
  (`KismetSystemLibrary.RetriggerableDelay` 0.5)
  (set `self.Rank Points` (`KismetMathLibrary.FClamp` (+ (`self.Rank Points`) (`self.Points To Add`)) (`self.Min Rank Points`) (`self.Max Rank Points`)))
  (set `self.Points To Add` 0.0))

(event `Update Level - Widget (Owner)`
  ;[0 0 0] Level - Update
  (`self.Update Level` (`self.Current Level`)))

(event `Update Experience - Widget`
  (params (`Current Experience` :type Integer) (`Target Experience` :type Integer))
  ;[0 0 0] Experience Progress Bar - Update (Owner)
  (`self.Update Experience` `Current Experience` `Target Experience`))

(event `Spawn Niagara`
  (params (InValue :type "LinearColor Structure (by ref)"))
  ;[0 0 0] Spawn Niagara - Multicast
  (if (not (`KismetSystemLibrary.IsDedicatedServer`))
    (bind _returnvalue (`NiagaraFunctionLibrary.SpawnSystemAttached` "/Game/SpellSystemV2/LevelingSystemX/Niagara/NS_EXP_Received.NS_EXP_Received" (`Character.CapsuleComponent` (`self.As Character`)) "None" (0.0 0.0 0.0) (struct) "KeepRelativeOffset" true))
    (`NiagaraComponent.SetVariableLinearColor` _returnvalue "EXP Received Color" InValue)))

(event `Update Rank`
  ;[0 0 0] Update Rank
  (bind (_last_rank_name_l1 _last_color_l1) (`self.Refresh Rank`))
  (bind _aswb_player_level_attached (cast `/Game/SpellSystemV2/LevelingSystemX/Blueprints/Widgets/WB_PlayerLevel_Attached` (`WidgetComponent.GetUserWidgetObject` (`self.Level and Rank - Widget`))))
  (`/Game/SpellSystemV2/LevelingSystemX/Blueprints/Widgets/WB_PlayerLevel_Attached.Update Rank` _aswb_player_level_attached _last_rank_name_l1 _last_color_l1))

(event `Refresh Widget Component`
  ;[0 0 0] Refresh widget with level, rank and player name
  (bind _level_and_rank___widget (`/Game/SpellSystemV2/LevelingSystemX/Blueprints/BP_Components_MacroLib.Get Level And Rank - Widget` 15.0 self)
    (:`Is Valid`
      (bind _aswb_player_level_attached (cast `/Game/SpellSystemV2/LevelingSystemX/Blueprints/Widgets/WB_PlayerLevel_Attached` (`WidgetComponent.GetUserWidgetObject` _level_and_rank___widget)))
      (`/Game/SpellSystemV2/LevelingSystemX/Blueprints/Widgets/WB_PlayerLevel_Attached.Update Level` _aswb_player_level_attached (`self.Current Level`)))))

(event `Add Experience + Visual Effect`
  (params (Experience :type Integer) (`Reward Level` :type Integer))
  ;[0 0 0] Add Experience + Visual Effect (Server)
  (bind _color (`self.Experience Color` `Reward Level`))
  (`self.Spawn Niagara` _color)
  (`self.Increase The Experience` Experience `Reward Level`))

(event `Set Widget Visibility (PlayerName,Lvl,Rank)`
  (params (`Overlaping Actor` :type "Actor Object Reference") (Visible :type Boolean))
  ;[0 0 0] Widget Visibility  (PlayerName, Rank, Level)
  (`/Engine/EditorBlueprintResources/StandardMacros.IsValid` (`Actor.GetComponentByClass` `Overlaping Actor` "BP_Player_LevelingSystemX_C")
    (:`Is Valid`
      (if (== `Overlaping Actor` (`self.GetOwner`))
        (bind _aswb_player_level_attached (cast `/Game/SpellSystemV2/LevelingSystemX/Blueprints/Widgets/WB_PlayerLevel_Attached` (`WidgetComponent.GetUserWidgetObject` (`self.Level and Rank - Widget`))))
        (`/Game/SpellSystemV2/LevelingSystemX/Blueprints/Widgets/WB_PlayerLevel_Attached.Render Opacity Animation` _aswb_player_level_attached true)
        (else
          (`KismetArrayLibrary.Array_Add` (`self.Overlaping Actor`) `Overlaping Actor`)
          (bind _level_and_rank___widget (`/Game/SpellSystemV2/LevelingSystemX/Blueprints/BP_Components_MacroLib.Get Level And Rank - Widget (Array)` 10.0 (`self.Overlaping Actor`))
            (:`Is Valid`
              (bind _aswb_player_level_attached_2 (cast `/Game/SpellSystemV2/LevelingSystemX/Blueprints/Widgets/WB_PlayerLevel_Attached` (`WidgetComponent.GetUserWidgetObject` _level_and_rank___widget)))
              (`/Game/SpellSystemV2/LevelingSystemX/Blueprints/Widgets/WB_PlayerLevel_Attached.Render Opacity Animation` _aswb_player_level_attached_2 Visible))
            (:`Complete`
              (`KismetArrayLibrary.Array_Clear` (`self.Overlaping Actor`)))))))))

(event `Add Experience - Server`
  (params (Experience :type Integer) (`Reward Level` :type Integer))
  ;[0 0 0] Add Experience (Server)
  (`self.Increase The Experience` Experience `Reward Level`))

(event `Debug Sphere -Multicast`
  ;[0.9619 1 0] Example Attack  --- Sphere Debug
  (`KismetSystemLibrary.DrawDebugSphere` (`Actor.K2_GetActorLocation` (`self.GetOwner`)) 111.0 12 (struct :`R` 1.0 :`G` 0.893594 :`A` 1.0) 0.2))

(event `Remove Experience - Server`
  (params (Experience :type Integer))
  ;[0 0 0] Remove Experience (Server)
  (`self.Decrease The Experience` Experience))

(event `Attack`
  (bind _as_character (`self.As Character`))
  ;[0.9619 1 0] Example Attack  --- Sphere Debug
  (`|ExecutionSequence`
    (:`then_0`
      (`self.Debug Sphere -Multicast`))
    (:`then_1`
      (bind _outactors (`KismetSystemLibrary.SphereOverlapActors` (`Actor.K2_GetActorLocation` (`self.GetOwner`)) 111.0 (`|MakeArray` "ObjectTypeQuery3" :!type "EObjectTypeQuery Enum") null (`|MakeArray` (`self.GetOwner`))))
      (for _array_element _outactors
        (`GameplayStatics.ApplyDamage` _array_element 55.0 (`Pawn.GetController` _as_character) _as_character)))))

(event `Add Rank Points - Server`
  (params (Points :type "Float (double-precision)"))
  ;[0 0 0] Add Rank Points (Server)
  (`self.Add Rank Points` Points))

(event `Remove Rank Points - Server`
  (params (Points :type "Float (double-precision)"))
  ;[0 0 0] Remove Rank Points (Server)
  (`self.Remove Rank Points` Points))

(fn `Add Rank Points`
  (params (Points :type "Float (double-precision)"))
  ;[0 0 0] Add Rank Points
  (set `self.Points To Add` (+ (`self.Points To Add`) Points))
  (`self.Refreshing Rank Points`))

(fn `BP_Player_LevelingSystemX_AutoGenFunc`
  (params (OverlappedComponent :type "PrimitiveComponent Object Reference") (OtherActor :type "Actor Object Reference") (OtherComp :type "PrimitiveComponent Object Reference") (OtherBodyIndex :type Integer) (bFromSweep :type Boolean) (SweepResult :type "HitResult Structure (by ref)"))
  ;[0 0 0] Begin Overlap - Sphere
  (`self.Set Widget Visibility (PlayerName,Lvl,Rank)` OtherActor true)
  (return))

(fn `BP_Player_LevelingSystemX_AutoGenFunc1`
  (params (OverlappedComponent :type "PrimitiveComponent Object Reference") (OtherActor :type "Actor Object Reference") (OtherComp :type "PrimitiveComponent Object Reference") (OtherBodyIndex :type Integer))
  ;[0 0 0] End Overlap - Sphere
  (`self.Set Widget Visibility (PlayerName,Lvl,Rank)` OtherActor)
  (return))

(fn `Calculate Experience`
  (params (Experience :type Integer) (`Reward Level` :type Integer))
  (returns (EXP :type Integer))
  (locals (`Reward Level L` :type Integer) (`Exp Local` :type Integer))
  ;[0 0 0] Calculate Experience
  (set `local.Exp Local` Experience)
  (bind _output_get (set `local.Reward Level L` `Reward Level`))
  (`self.The Power Of Experience` _output_get
    (:`>`
      (set `local.Exp Local` (* (`KismetMathLibrary.Clamp` (`local.Exp Local`) 1 46340) (`KismetMathLibrary.FTrunc` (`KismetMathLibrary.FClamp` (* (`KismetMathLibrary.Conv_IntToDouble` (- (+ (`local.Reward Level L`) 1) (`self.Current Level`))) 1.125) 1.0 463400.0))))
      (return (`local.Exp Local`)))
    (:`<`
      (set `local.Exp Local` (`KismetMathLibrary.Clamp` (`KismetMathLibrary.FTrunc` (/ (`local.Exp Local`) (* (`KismetMathLibrary.Conv_IntToDouble` (- (`self.Current Level`) (`local.Reward Level L`))) 1.125))) 1 46340))
      (return (`local.Exp Local`)))
    (:`==`
      (return (`local.Exp Local`)))))

(fn `Decrease The Experience`
  (params (Experience :type Integer))
  (locals (`Initial level L` :type Integer) (`End Level L` :type Integer))
  (bind _returnvalue (- (`self.Current Experience`) Experience))
  ;[0 0 0] Decrease The Experience
  (set `self.Current Experience` (`KismetMathLibrary.Clamp` (`KismetMathLibrary.SelectInt` 0 _returnvalue (and (< _returnvalue 0) (<= (`self.Current Level`) 1))) 0 (`self.Target Experience`)))
  ;;[0 0 0] Experience Progress Bar - Update
  (`self.Update Experience - Widget` (`self.Current Experience`) (`self.Target Experience`))
  (return))

(fn `Experience Color`
  (params (`Revard Level` :type Integer))
  (returns (Color :type "LinearColor Structure"))
  ;[0 0 0] Experience Color
  (`self.The Power Of Experience` `Revard Level`
    (:`>`
      (set `self.Color Index` 0))
    (:`<`
      (set `self.Color Index` 1))
    (:`==`
      (set `self.Color Index` 2)))
  (bind _color (`self.Get Experience Color` (`self.Color Index`)))
  (return _color))

(fn `Get Experience Color`
  (params (Index :type Integer))
  (returns (Color :type "LinearColor Structure"))
  ;[0 0 0] Get Color
  (switch `int` Index
    (:`0`
      (return (`.>_9_9AEA98BC44CB188084F6999C4FC12A17` (break `/Game/SpellSystemV2/LevelingSystemX/Structures/S_ExperienceColor` (`self.EXP Color`)))))
    (:`1`
      (return (`.<_8_B2413C474A567730562A4A9DA30B8F3C` (break `/Game/SpellSystemV2/LevelingSystemX/Structures/S_ExperienceColor` (`self.EXP Color`)))))
    (:`2`
      (return (`.None_6_8DD224BE4FD5C44EE9536C97B78E2D3F` (break `/Game/SpellSystemV2/LevelingSystemX/Structures/S_ExperienceColor` (`self.EXP Color`)))))))

(fn `Increase The Experience`
  (params (Experience :type Integer) (`Reward Level` :type Integer))
  (locals (`Exp (Local)` :type Integer) (`Enemy Level L` :type Integer))
  ;[0 0 0] Increase The Experience
  (if (not (== (`self.Max Experience`) (`self.Current Experience`)))
    (bind _exp (`self.Calculate Experience` (`local.Experience`) (`local.Reward Level`)))
    (`self.Leveling` _exp (`local.Reward Level`))
    (return)))

(fn `Leveling`
  (params (Exp :type Integer) (`Reward Level` :type Integer))
  (locals (`Initial level L` :type Integer :default 0) (`End Level L` :type Integer :default 0) (`Spell Points L` :type Integer :default 0))
  (bind _returnvalue (`Actor.GetComponentByClass` (`self.GetOwner`) "/Game/SpellSystemV2/SpellSystem/Blueprints/SpellSystem_Component.SpellSystem_Component_C"))
  (bind _returnvalue_2 (+ (`self.Current Experience`) Exp))
  ;[0 0 0] Leveling
  (set `self.Current Experience` (`KismetMathLibrary.SelectInt` (`self.Max Experience`) _returnvalue_2 (and (< _returnvalue_2 0) (>= (`self.Current Level`) (`self.Max Level`)))))
  (set `local.Initial level L` (`self.Current Level`))
  (if (>= (`self.Current Level`) (`self.Max Level`))
    (if (>= (`self.Current Experience`) (`self.Target Experience`))
      (set `self.Current Experience` (`self.Max Experience`)))
    ;;[0 0 0] Experience Progress Bar - Update
    (`self.Update Experience - Widget` (`self.Current Experience`) (`self.Target Experience`))
    (else
      (set `local.End Level L` (`self.Current Level`))
      (if (>= (`self.Current Experience`) (`self.Target Experience`)) :!label _label
        ;;[0 0 0] Level UP
        (set `local.End Level L` (`KismetMathLibrary.Clamp` (+ (`local.End Level L`) 1) 1 (`self.Max Level`)))
        ;;[0.8964 1 0] Spell System
        (set `local.Spell Points L` (+ (`local.Spell Points L`) 1))
        ;;[0 0 0] Set New Goal
        (set `self.Current Experience` (- (`self.Current Experience`) (`self.Target Experience`)))
        (set `self.Target Experience` (`KismetMathLibrary.SelectInt` (`self.Max Experience`) (+ (`self.Target Experience`) (* (`self.Current Level`) 100)) (== (`self.Current Level`) (`self.Max Level`))))
        (goto _label)
        (else
          ;;[0.8964 1 0] Spell System
          (`/Engine/EditorBlueprintResources/StandardMacros.IsValid` _returnvalue
            (:`Is Valid`
              (`/Game/SpellSystemV2/SpellSystem/Blueprints/SpellSystem_Component.Set Spell Points` _returnvalue (`local.Spell Points L`)))
            (:`Is Not Valid`
              _))
          (if (not (== (`local.End Level L`) (`local.Initial level L`)))
            ;;[0 0 0] Level - Update
            (set `self.Current Level` (`local.End Level L`))
            (`self.Leveling Up (Visual Effect) - Server`))
          ;;[0 0 0] Experience Progress Bar - Update
          (`self.Update Experience - Widget` (`self.Current Experience`) (`self.Target Experience`))
          (return))))))

(fn `OnRep_Current Level`
  ;[0 0 0] Update Level
  (`self.Update Level` (`self.Current Level`))
  (`self.Refresh Widget Component`))

(fn `OnRep_Player Name`
  ;[0 0 0] Set Player Name
  (`self.Set Name` (`self.Player Name`)))

(fn `OnRep_Rank Points`
  ;[0 0 0] Update Rank
  (`self.Level and Rank - Widget`
    (:`then`
      (`self.Update Rank`))
    (:`else`)))

(fn `Refresh Rank`
  (returns (`Last Rank Name L1` :type Text) (`Last Color L1` :type "LinearColor Structure"))
  (locals (`Last Rank Name L` :type Text) (`Last Color L` :type "LinearColor Structure"))
  ;[0 0 0] Refresh Level
  (for _array_element (`self.Rank`)
    (bind (_rankname _requiredpoints _color) (break `/Game/SpellSystemV2/LevelingSystemX/Structures/S_Rank` _array_element))
    (if (>= (`self.Rank Points`) _requiredpoints)
      (set `local.Last Rank Name L` _rankname)
      (set `local.Last Color L` _color)
      (break)))
  (return (`local.Last Rank Name L`) (`local.Last Color L`)))

(fn `Remove Rank Points`
  (params (Points :type "Float (double-precision)"))
  ;[0 0 0] Remove Rank Points
  (set `self.Points To Add` (- (`self.Points To Add`) Points))
  (`self.Refreshing Rank Points`))

(fn `Set Collision`
  (bind _sphere_collision (`self.Sphere Collision`))
  ;[0 0 0] Set Collision
  (bind _returnvalue (`|AddComponentByClass` (`self.As Character`) "/Script/Engine.SphereComponent" false (`KismetMathLibrary.MakeTransform` (0.0 0.0 0.0))))
  (bind _output_get (set `self.Sphere Collision` _returnvalue))
  (`SphereComponent.SetSphereRadius` _output_get (`self.Widget Visibility Radius`) true)
  (`PrimitiveComponent.SetCollisionResponseToAllChannels` (`self.Sphere Collision`) "ECR_Ignore")
  (`PrimitiveComponent.SetCollisionEnabled` (`self.Sphere Collision`) "QueryOnly")
  (`PrimitiveComponent.SetCollisionResponseToChannel` _sphere_collision "ECC_Pawn" "ECR_Overlap")
  (add `PrimitiveComponent.OnComponentBeginOverlap` _sphere_collision (`|CreateDelegate` :!event `BP_Player_LevelingSystemX_AutoGenFunc`))
  (add `PrimitiveComponent.OnComponentEndOverlap` (`self.Sphere Collision`) (`|CreateDelegate` :!event `BP_Player_LevelingSystemX_AutoGenFunc1`))
  (for _array_element (`PrimitiveComponent.GetOverlappingActors` (`self.Sphere Collision`) "/Script/Engine.Actor")
    (`self.Set Widget Visibility (PlayerName,Lvl,Rank)` _array_element true))
  (return))

(fn `Set Level and Rank - Widget`
  (locals (`Skeletal Mesh` :type "SkeletalMeshComponent Object Reference"))
  ;[0 0 0] Set Level And Rank - Widget
  (bind _returnvalue (`|AddComponentByClass` :`self` (`self.As Character`) :`Class` "/Script/UMG.WidgetComponent"))
  (bind _output_get (set `self.Level and Rank - Widget` _returnvalue))
  (`SceneComponent.K2_AttachToComponent` _output_get (`Character.Mesh` (`self.As Character`)) "head" "SnapToTarget" "SnapToTarget" "KeepRelative" true)
  (`SceneComponent.K2_SetRelativeLocation` _output_get (`self.Widget Location`) false false)
  (bind _returnvalue_2 (`|CreateWidget` "/Game/SpellSystemV2/LevelingSystemX/Blueprints/Widgets/WB_PlayerLevel_Attached.WB_PlayerLevel_Attached_C"))
  (bind (_last_rank_name_l1 _last_color_l1) (`self.Refresh Rank`))
  (`/Game/SpellSystemV2/LevelingSystemX/Blueprints/Widgets/WB_PlayerLevel_Attached.Update Rank` _returnvalue_2 _last_rank_name_l1 _last_color_l1)
  (`/Game/SpellSystemV2/LevelingSystemX/Blueprints/Widgets/WB_PlayerLevel_Attached.Update Level` _returnvalue_2 (`self.Current Level`))
  (`WidgetComponent.SetWidget` (`self.Level and Rank - Widget`) _returnvalue_2)
  (`WidgetComponent.SetWidgetSpace` (`self.Level and Rank - Widget`) "Screen")
  (`WidgetComponent.SetDrawAtDesiredSize` (`self.Level and Rank - Widget`) true)
  (return))

(fn `Set Player Name`
  (params (`Player Name` :type Name))
  (`self.Set Name` `Player Name`))