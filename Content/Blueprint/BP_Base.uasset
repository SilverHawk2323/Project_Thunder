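; BP_Base is a base actor with a team number that switches sides when its health runs out.
; A DoOnce binds DamageTaken to the OnDeath of the first BP_EnemyBase overlapping its Box.
; Each call subtracts fixed health from BPCDamageSystem; at zero it swaps teams 1 and 2, refills health and prints a message.
; Damage, health and team query functions are stubs returning default values.
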(event `self.Box.OnComponentBeginOverlap`
  (params (OverlappedComponent :type "PrimitiveComponent Object Reference") (OtherActor :type "Actor Object Reference") (OtherComp :type "PrimitiveComponent Object Reference") (OtherBodyIndex :type Integer) (bFromSweep :type Boolean) (SweepResult :type "HitResult Structure (by ref)"))
  (bind _asbp_enemy_base (cast `/Game/Blueprint/AI/Enemy/BP_EnemyBase` OtherActor))
  (`/Engine/EditorBlueprintResources/StandardMacros.DoOnce` false
    (:`Completed`
      (add `/Game/Blueprint/AI/Enemy/BP_EnemyBase.OnDeath` _asbp_enemy_base (delegate `DamageTaken`)))))

(event `DamageTaken`
  (bind _bpc_damagesystem (`self.BPC_DamageSystem`))
  (bind _output_get (set `/Game/Blueprint/DamageSystem/BPC_DamageSystem.Health` (- (`/Game/Blueprint/DamageSystem/BPC_DamageSystem.Health` (`self.BPC_DamageSystem`)) 5.0) (`self.BPC_DamageSystem`)))
  (if (<= _output_get 0.0)
    (set `self.TeamNumber` (select `int` (`self.TeamNumber`) :`0` 0 :`1` 2 :`2` 1))
    (set `/Game/Blueprint/DamageSystem/BPC_DamageSystem.Health` (`/Game/Blueprint/DamageSystem/BPC_DamageSystem.MaxHealth` _bpc_damagesystem) _bpc_damagesystem)
    (`KismetSystemLibrary.PrintString` "Based Switched Sides")))

(fn `GetCurrentHealth`
  (returns (Health :type "Float (double-precision)"))
  (return 0.0))

(fn `GetMaxHealth`
  (returns (MaxHealth :type "Float (double-precision)"))
  (return 0.0))

(fn `GetTeamNumber`
  (returns (TeamNumber :type Integer))
  (return 0))

(fn `Heal`
  (params (Amount :type "Float (double-precision)"))
  (returns (`New Health` :type "Float (double-precision)"))
  (return 0.0))

(fn `IsAttacking`
  (returns (Attacking :type Boolean))
  (return false))

(fn `IsDead`
  (returns (Dead :type Boolean))
  (return false))

(fn `ReserveAttackToken`
  (params (Amount :type Integer))
  (returns (Success :type Boolean))
  (return false))

(fn `TakeDamage`
  (params (DamageInfo :type "/Game/Blueprint/DamageSystem/S_DamageInfo Structure") (`Damage Causer` :type "Actor Object Reference"))
  (returns (WasDamaged :type Boolean))
  (return false))

(fn `UserConstructionScript`)