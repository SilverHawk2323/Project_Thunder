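; Boss enemy character that extends a parent enemy Blueprint with high health and a smash attack.
; Construction fills the damage component's health to its maximum, and Attack runs the parent logic before triggering the attack component's boss smash with AttackInfo.
; WeakonBoss halves current health and replaces AttackInfo with a parryable, force-interrupting hit.
; It sets its own attack and defend ranges, while other overrides simply forward to the parent.
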(event `/Game/Blueprint/DamageSystem/BPI_Damageable.ReturnAttackToken`
  (params (Amount :type Integer))
  (`parent.ReturnAttackToken` Amount))

(event `/Game/Blueprint/AI/Enemy/BPI_EnemyAI.AttackEnd`
  (params (AttackTarget :type "Actor Object Reference"))
  (`parent.AttackEnd` AttackTarget))

(event `/Game/Blueprint/AI/Enemy/BPI_EnemyAI.StoreAttackTokens`
  (params (AttackTarget :type "Actor Object Reference") (Amount :type Integer))
  (`parent.StoreAttackTokens` AttackTarget Amount))

(event `/Game/Blueprint/AI/Enemy/BPI_EnemyAI.Attack`
  (params (AttackTarget :type "Actor Object Reference"))
  (`parent.Attack` AttackTarget)
  (`/Game/Blueprint/DamageSystem/Attacks/BPC_Attacks.BossSmashAttack` (`self.BPC_Attacks`) self (`self.Attack Info`)))

(event `WeakonBoss`
  (bind _bpc_damagesystem (`self.BPC_DamageSystem`))
  (set `/Game/Blueprint/DamageSystem/BPC_DamageSystem.Health` (* (`/Game/Blueprint/DamageSystem/BPC_DamageSystem.Health` _bpc_damagesystem) 0.5) _bpc_damagesystem)
  (set `self.Attack Info` (make `/Game/Blueprint/DamageSystem/S_DamageInfo` 25.0 "NewEnumerator1" "NewEnumerator1" false false true true)))

(fn `AttackStart`
  (params (AttackTarget :type "Actor Object Reference") (TokensNeeded :type Integer))
  (returns (Success :type Boolean))
  (bind _success (`parent.AttackStart` AttackTarget TokensNeeded))
  (return _success))

(fn `GetCurrentHealth`
  (returns (Health :type "Float (double-precision)"))
  (bind _health (`parent.GetCurrentHealth`))
  (return _health))

(fn `GetIdealRange`
  (returns (AttackRadius :type "Float (double-precision)") (DefendRadius :type "Float (double-precision)"))
  (`parent.GetIdealRange`)
  (return 200.0 400.0))

(fn `GetMaxHealth`
  (returns (MaxHealth :type "Float (double-precision)"))
  (bind _maxhealth (`parent.GetMaxHealth`))
  (return _maxhealth))

(fn `GetPatrolRoute`
  (returns (PatrolRoute :type "/Game/Blueprint/AI/BP_PatrolRoute Object Reference"))
  (bind _patrolroute (`parent.GetPatrolRoute`))
  (return _patrolroute))

(fn `GetTeamNumber`
  (returns (TeamNumber :type Integer))
  (bind _teamnumber (`parent.GetTeamNumber`))
  (return _teamnumber))

(fn `Heal`
  (params (Amount :type "Float (double-precision)"))
  (returns (`New Health` :type "Float (double-precision)"))
  (bind _new_health (`parent.Heal` Amount))
  (return _new_health))

(fn `IsAttacking`
  (returns (Attacking :type Boolean))
  (bind _attacking (`parent.IsAttacking`))
  (return _attacking))

(fn `IsDead`
  (returns (Dead :type Boolean))
  (bind _dead (`parent.IsDead`))
  (return _dead))

(fn `ReserveAttackToken`
  (params (Amount :type Integer))
  (returns (Success :type Boolean))
  (bind _success (`parent.ReserveAttackToken` Amount))
  (return _success))

(fn `SetMovementSpeed`
  (params (Speed :type "/Game/Blueprint/AI/Enums/E_MovementSpeed Enum" :default "NewEnumerator2"))
  (returns (SpeedValue :type "Float (double-precision)"))
  (bind _speedvalue (`parent.SetMovementSpeed` Speed))
  (return _speedvalue))

(fn `TakeDamage`
  (params (DamageInfo :type "/Game/Blueprint/DamageSystem/S_DamageInfo Structure") (`Damage Causer` :type "Actor Object Reference"))
  (returns (WasDamaged :type Boolean))
  (bind _wasdamaged (`parent.TakeDamage` DamageInfo `Damage Causer`))
  (return _wasdamaged))

(fn `UserConstructionScript`
  (bind _bpc_damagesystem (`self.BPC_DamageSystem`))
  (`parent.UserConstructionScript`)
  (bind _output_get (set `/Game/Blueprint/DamageSystem/BPC_DamageSystem.MaxHealth` 1000.0 _bpc_damagesystem))
  (set `/Game/Blueprint/DamageSystem/BPC_DamageSystem.Health` _output_get _bpc_damagesystem))