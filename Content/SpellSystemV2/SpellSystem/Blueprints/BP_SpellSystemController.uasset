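; Player controller for the spell system that creates the spell HUD for the local player and connects it to the controlled pawn.
; On BeginPlay it hands the HUD's spell widget to the pawn's SpellSystem_Component and calls SetSpells, retrying on a timer until a pawn exists.
; A missing component prints an on-screen warning.
; Left Ctrl toggles the component's input block, the mouse cursor and the Game/UI input mode.
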(event `self.ReceiveBeginPlay`
  ;[0 0 0] Begin Play
  (if (`self.IsLocalPlayerController`)
    (bind _returnvalue (`|CreateWidget` "/Game/SpellSystemV2/SpellSystem/Blueprints/Widgets/WB_HUD_SpellSystem.WB_HUD_SpellSystem_C" self))
    (set `self.HUD` _returnvalue)
    (`UserWidget.AddToViewport` _returnvalue 0)
    (`self.Set Spells`)))

(event `CustomEvent`
  (bind _returnvalue (`self.K2_GetPawn`))
  (bind _returnvalue_2 (`self.GetComponentByClass` _returnvalue "/Game/SpellSystemV2/SpellSystem/Blueprints/SpellSystem_Component.SpellSystem_Component_C"))
  ;[0 0 0] Set Spells - Owning Client
  (`/Engine/EditorBlueprintResources/StandardMacros.IsValid` _returnvalue :!label _label
    (:`Is Valid`
      (`/Engine/EditorBlueprintResources/StandardMacros.IsValid` _returnvalue_2
        (:`Is Valid`
          (set `/Game/SpellSystemV2/SpellSystem/Blueprints/SpellSystem_Component.SpellSystem_Widget` (`/Game/SpellSystemV2/SpellSystem/Blueprints/Widgets/WB_HUD_SpellSystem.W_SpellSystem_Widget` (`self.HUD`)) _returnvalue_2)
          (`/Game/SpellSystemV2/SpellSystem/Blueprints/SpellSystem_Component.Set Spells` _returnvalue_2)
          (`WidgetBlueprintLibrary.SetInputMode_GameOnly` self))
        (:`Is Not Valid`
          (`KismetSystemLibrary.PrintString` "Add Spell System Component To Your Character" true true (struct :`R` 1.0 :`A` 1.0) 52.0))))
    (:`Is Not Valid`
      (`KismetSystemLibrary.K2_SetTimerDelegate` (delegate `CustomEvent`) 0.5))))

(event `Set Spells`
  ;[0 0 0] Set Spells - Owning Client
  (goto _label))

(event `Key|LeftControl`
  (params (Key :type "Key Structure"))
  (bind _returnvalue (`self.GetComponentByClass` (`self.K2_GetPawn` self) "/Game/SpellSystemV2/SpellSystem/Blueprints/SpellSystem_Component.SpellSystem_Component_C"))
  ;[0 0 0] Left Ctrl
  (:`Pressed`
    (if (`/Game/SpellSystemV2/SpellSystem/Blueprints/SpellSystem_Component.Block Input` (`self.GetComponentByClass` (`self.K2_GetPawn` self) "/Game/SpellSystemV2/SpellSystem/Blueprints/SpellSystem_Component.SpellSystem_Component_C"))
      (set `/Game/SpellSystemV2/SpellSystem/Blueprints/SpellSystem_Component.Block Input` false _returnvalue)
      (set `self.bShowMouseCursor` false)
      (`WidgetBlueprintLibrary.SetInputMode_GameOnly` self)
      (else
        (set `/Game/SpellSystemV2/SpellSystem/Blueprints/SpellSystem_Component.Block Input` true _returnvalue)
        (set `self.bShowMouseCursor` true)
        (`WidgetBlueprintLibrary.SetInputMode_GameAndUIEx` self (`self.HUD`))))))

(fn `UserConstructionScript`)