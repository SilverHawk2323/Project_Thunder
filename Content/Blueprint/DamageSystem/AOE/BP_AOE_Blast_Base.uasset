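; Base Blueprint for an area-of-effect blast in the damage system, adding visual and audio feedback on top of its parent's Trigger logic.
; Trigger calls the parent, then spawns the BlastEffect system attached to the root and plays BlastSound at the actor's location.
; The actor destroys itself when the effect system finishes, or after a short delay if no valid effect is set.
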(event `self.Trigger`
  (`parent.Trigger`)
  (`self.SpawnBlastEffect`)
  (`self.SpawnBlastSound`))

(event `SpawnBlastEffect`
  (bind _blast_effect (`self.Blast Effect`)
    (:`then`
      (bind _returnvalue (`NiagaraFunctionLibrary.SpawnSystemAttached` _blast_effect (`self.DefaultSceneRoot`) "None" (0.0 0.0 0.0) (struct) "KeepRelativeOffset"))
      (add `NiagaraComponent.OnSystemFinished` _returnvalue (delegate `SystemFinishedEvent`)))
    (:`else`
      (`KismetSystemLibrary.Delay` 1.0)
      (`self.K2_DestroyActor`))))

(event `SystemFinishedEvent`
  (params (PSystem :type "NiagaraComponent Object Reference"))
  (`self.K2_DestroyActor`))

(event `SpawnBlastSound`
  (bind _blast_sound (`self.Blast Sound`)
    (:`then`
      (`GameplayStatics.PlaySoundAtLocation` _blast_sound (`self.K2_GetActorLocation`) (struct) 1.0 1.0 0.0 null null null null))
    (:`else`)))

(fn `UserConstructionScript`
  (`parent.UserConstructionScript`))