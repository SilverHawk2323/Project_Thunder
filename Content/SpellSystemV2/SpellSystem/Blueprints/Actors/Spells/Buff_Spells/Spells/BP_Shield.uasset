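; BP_Shield is a buff spell actor that surrounds its caster with a temporary, fading shield sphere.
; On begin play the server attaches it to the instigator's root and sets Forward, whose OnRep creates the dynamic material and plays an opacity timeline.
; After a timed hold, Forward clears to reverse the fade, then the server notifies the caster's SpellSystem_Component and destroys the actor.
; The sphere's overlap check currently triggers no action.
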(event `self.ReceiveBeginPlay`
  ;[0 0 0] Begin Play
  (`parent.ReceiveBeginPlay`)
  (if (`KismetSystemLibrary.IsServer`)
    (`self.K2_AttachToActor` self (`self.GetInstigator`) "root" "SnapToTarget" "SnapToTarget" "SnapToTarget" false)
    (set `self.Forward` true)))

(event `self.Sphere1.OnComponentBeginOverlap`
  (params (OverlappedComponent :type "PrimitiveComponent Object Reference") (OtherActor :type "Actor Object Reference") (OtherComp :type "PrimitiveComponent Object Reference") (OtherBodyIndex :type Integer) (bFromSweep :type Boolean) (SweepResult :type "HitResult Structure (by ref)"))
  ;[0 0 0] Sphere - Overlap
  (if (!= (`self.GetInstigator` OtherActor) (`self.GetInstigator`))
    _))

(event `Shield Opacity - All`
  ;[0 0 0] Shield Opacity
  (if (`self.Forward`)
    (bind (_direction _opacity) (`Timeline|Timeline` :!label _label)
      (:`Update`
        (`MaterialInstanceDynamic.SetScalarParameterValue` (`self.Dynamic Material`) "Opacity" _opacity))
      (:`Finished`
        (if (`KismetSystemLibrary.IsServer`)
          (if (`self.Forward`)
            (`KismetSystemLibrary.K2_SetTimerDelegate` (delegate `CustomEvent`) 5.0)
            (else
              (`/Game/SpellSystemV2/SpellSystem/Blueprints/SpellSystem_Component.Spell Response - Server` (`self.GetComponentByClass` (`self.GetInstigator`) "/Game/SpellSystemV2/SpellSystem/Blueprints/SpellSystem_Component.SpellSystem_Component_C") (`self.Spell Name`))
              (`self.K2_DestroyActor`))))))
    (else
      (goto _label :!via `Reverse`))))

(event `CustomEvent`
  ;[0 0 0] Shield Opacity
  (set `self.Forward` false))

(fn `OnRep_Forward`
  (bind _returnvalue (`PrimitiveComponent.CreateDynamicMaterialInstance` (`self.Sphere1`) 0 "/Game/SpellSystemV2/SpellSystem/Materials/M_Shield.M_Shield" "None"))
  (set `self.Dynamic Material` _returnvalue)
  (`self.Shield Opacity - All`))

(fn `UserConstructionScript`
  (`parent.UserConstructionScript`))