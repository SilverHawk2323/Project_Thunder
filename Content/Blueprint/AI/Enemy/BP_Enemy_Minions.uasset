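; BP_Enemy_Minions is a melee minion enemy, a child of a base enemy Blueprint, linked to a Captain.
; Attack runs the parent logic, then triggers a single light attack through the BPCAttacks component with its own damage info, and DamageResponse resets that combo.
; It overrides its ideal attack and defend ranges and exposes GetCaptain, which prints a warning when none is assigned.
; Token, health, team, movement and patrol functions just forward to the parent.
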(event `/Game/Blueprint/AI/Enemy/BPI_EnemyAI.Attack`
  (params (AttackTarget :type "Actor Object Reference"))
  (`parent.Attack` AttackTarget)
  (`/Game/Blueprint/DamageSystem/Attacks/BPC_Attacks.LightAttack` (`self.BPC_Attacks`) 1 (make `/Game/Blueprint/DamageSystem/S_DamageInfo` 10.0 "NewEnumerator1" "NewEnumerator1") self))

(event `/Game/Blueprint/AI/Enemy/BPI_EnemyAI.AttackEnd`
  (params (AttackTarget :type "Actor Object Reference"))
  (`parent.AttackEnd` AttackTarget))

(event `self.DamageResponse`
  (params (DamageResponse :type "/Game/Blueprint/DamageSystem/E_DamageResponse Enum" :default "NewEnumerator0") (DamageCauser :type "Actor Object Reference"))
  (`parent.DamageResponse` DamageResponse DamageCauser)
  (`/Game/Blueprint/DamageSystem/Attacks/BPC_Attacks.ResetCombo` (`self.BPC_Attacks`)))

(event `/Game/Blueprint/DamageSystem/BPI_Damageable.ReturnAttackToken`
  (params (Amount :type Integer))
  (`parent.ReturnAttackToken` Amount))

(event `/Game/Blueprint/AI/Enemy/BPI_EnemyAI.StoreAttackTokens`
  (params (AttackTarget :type "Actor Object Reference") (Amount :type Integer))
  (`parent.StoreAttackTokens` AttackTarget Amount))

(fn `AttackStart`
  (params (AttackTarget :type "Actor Object Reference") (TokensNeeded :type Integer))
  (returns (Success :type Boolean))
  (bind _success (`parent.AttackStart` AttackTarget TokensNeeded))
  (return _success))

(fn `GetCaptain`
  (returns (Captain :type "/Game/Blueprint/AI/Enemy/BP_EnemyBase Object Reference"))
  (bind _captain (`self.Captain`)
    (:`then`
      (return _captain))
    (:`else`
      (`KismetSystemLibrary.PrintString` "No Assigned Captain")
      (return null))))

(fn `GetCurrentHealth`
  (returns (Health :type "Float (double-precision)"))
  (bind _health (`parent.GetCurrentHealth`))
  (return _health))

(fn `GetIdealRange`
  (returns (AttackRadius :type "Float (double-precision)") (DefendRadius :type "Float (double-precision)"))
  (return 100.0 400.0))

(fn `GetMaxHealth`
  (returns (MaxHealth :type "Float (double-precision)"))
  (bind _maxhealth (`parent.GetMaxHealth`))
  (return _maxhealth))

(fn `GetPatrolRoute`
  (returns (PatrolRoute :type "/Game/Blueprint/AI/BP_PatrolRoute Object Reference"))
  (bind _patrolroute (`parent.GetPatrolRoute`))
  (return _patrolroute))

(fn `GetTeamNumber`
  (returns (TeamNumber :type Integer))
  (bind _teamnumber (`parent.GetTeamNumber`))
  (return _teamnumber))

(fn `Heal`
  (params (Amount :type "Float (double-precision)"))
  (returns (`New Health` :type "Float (double-precision)"))
  (bind _new_health (`parent.Heal` Amount))
  (return _new_health))

(fn `IsAttacking`
  (returns (Attacking :type Boolean))
  (bind _attacking (`parent.IsAttacking`))
  (return _attacking))

(fn `IsDead`
  (returns (Dead :type Boolean))
  (bind _dead (`parent.IsDead`))
  (return _dead))

(fn `ReserveAttackToken`
  (params (Amount :type Integer))
  (returns (Success :type Boolean))
  (bind _success (`parent.ReserveAttackToken` Amount))
  (return _success))

(fn `SetMovementSpeed`
  (params (Speed :type "/Game/Blueprint/AI/Enums/E_MovementSpeed Enum" :default "NewEnumerator2"))
  (returns (SpeedValue :type "Float (double-precision)"))
  (bind _speedvalue (`parent.SetMovementSpeed` Speed))
  (return _speedvalue))

(fn `TakeDamage`
  (params (DamageInfo :type "/Game/Blueprint/DamageSystem/S_DamageInfo Structure") (`Damage Causer` :type "Actor Object Reference"))
  (returns (WasDamaged :type Boolean))
  (bind _wasdamaged (`parent.TakeDamage` DamageInfo `Damage Causer`))
  (return _wasdamaged))

(fn `UserConstructionScript`
  (`parent.UserConstructionScript`))